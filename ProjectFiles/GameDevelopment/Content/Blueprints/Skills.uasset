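; Skills area actor that opens the player's skill UI while the Main character stands inside its box.
; On BeginPlay it enables input and adds a Nav widget pointing at itself.
; Box overlap calls WallRunFP, shows the skill widget and mouse cursor, and leaving calls WallRunTP and hides both.
; The overlap also toggles a gate on the F key, but nothing follows that gate.
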(event OnComponentBeginOverlap(Box)
  (params (OverlappedComponent :type Primitive%20Component%20Object%20Reference) (OtherActor :type Actor%20Object%20Reference) (OtherComp :type Primitive%20Component%20Object%20Reference) (OtherBodyIndex :type Integer) (bFromSweep :type Boolean) (SweepResult :type Hit%20Result%20Structure%20%28by%20ref%29))
  ;[0.9957 0 1] Access
  (bind _asmain (Utilities|Casting|CastToMain OtherActor))
  (Default|WallRunFP _asmain)
  (Default|ShowSkill (Variables|/Game/Blueprints/PlayerBlueprints/Main.Main_C|GetSkillWidget _asmain))
  (Variables|/Script/Engine.PlayerController|SetbShowMouseCursor (Game|GetPlayerController 0) true)
  (Utilities|FlowControl|Gate true) ; enters at Open
)

(event OnComponentEndOverlap(Box)
  (params (OverlappedComponent :type Primitive%20Component%20Object%20Reference) (OtherActor :type Actor%20Object%20Reference) (OtherComp :type Primitive%20Component%20Object%20Reference) (OtherBodyIndex :type Integer))
  ;[0.9957 0 1] Access
  (bind _asmain (Utilities|Casting|CastToMain OtherActor))
  (Default|WallRunTP _asmain)
  (Default|HideSkill (Variables|/Game/Blueprints/PlayerBlueprints/Main.Main_C|GetSkillWidget (stale OnComponentBeginOverlap(Box) _asmain)))
  (Variables|/Script/Engine.PlayerController|SetbShowMouseCursor (Game|GetPlayerController 0) false)
  (Utilities|FlowControl|Gate true) ; enters at Close
)

(event EventBeginPlay
  (bind _returnvalue (Game|GetPlayerController 0))
  ;[1 0 0.6676] Begin Play
  (Input|EnableInput _returnvalue)
  (bind _returnvalue_2 (UserInterface|CreateWidget "/Game/Blueprints/PlayerBlueprints/Nav.Nav_C" _returnvalue 2))
  (Variables|Default|SetWarningIcon _returnvalue_2)
  (Variables|/Game/Blueprints/PlayerBlueprints/Nav.Nav_C|SetArea _returnvalue_2 self)
  (UserInterface|Viewport|AddtoViewport _returnvalue_2 0))

(event Input|KeyboardEvents|F
  (params (Key :type Key%20Structure))
  ;[0.9957 0 1] Access
  (:Pressed
    (Utilities|FlowControl|Gate true)))

(fn ConstructionScript)