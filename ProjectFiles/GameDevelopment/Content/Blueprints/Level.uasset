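; Interactive area actor that lets the player switch the view to a designated camera while standing inside its trigger box.
; On BeginPlay it enables input and adds a Nav widget that holds a reference back to it.
; Box overlap calls WallRunFP or WallRunTP on the Main character and opens or closes a Gate, so F blends to MainCam only inside the box.
; The P key handler only casts the player character and does nothing further.
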(event OnComponentBeginOverlap(Box)
  (params (OverlappedComponent :type Primitive%20Component%20Object%20Reference) (OtherActor :type Actor%20Object%20Reference) (OtherComp :type Primitive%20Component%20Object%20Reference) (OtherBodyIndex :type Integer) (bFromSweep :type Boolean) (SweepResult :type Hit%20Result%20Structure%20%28by%20ref%29))
  ;[0.9957 0 1] Access
  (bind _asmain (Utilities|Casting|CastToMain OtherActor))
  (Default|WallRunFP _asmain)
  (Utilities|FlowControl|Gate true) ; enters at Open
)

(event OnComponentEndOverlap(Box)
  (params (OverlappedComponent :type Primitive%20Component%20Object%20Reference) (OtherActor :type Actor%20Object%20Reference) (OtherComp :type Primitive%20Component%20Object%20Reference) (OtherBodyIndex :type Integer))
  ;[0.9957 0 1] Access
  (bind _asmain (Utilities|Casting|CastToMain OtherActor))
  (Default|WallRunTP _asmain)
  (Utilities|FlowControl|Gate true) ; enters at Close
)

(event EventBeginPlay
  (bind _returnvalue (Game|GetPlayerController 0))
  ;[1 0 0.6676] Begin Play
  (Input|EnableInput _returnvalue)
  (bind _returnvalue_2 (UserInterface|CreateWidget "/Game/Blueprints/PlayerBlueprints/Nav.Nav_C" _returnvalue))
  (Variables|Default|SetWarningIcon _returnvalue_2)
  (Variables|/Game/Blueprints/PlayerBlueprints/Nav.Nav_C|SetArea _returnvalue_2 self)
  (UserInterface|Viewport|AddtoViewport _returnvalue_2 0))

(event Input|KeyboardEvents|F
  (params (Key :type Key%20Structure))
  ;[0.9957 0 1] Access
  (:Pressed
    (Utilities|FlowControl|Gate true
      (:Exit
        (Game|Player|SetViewTargetwithBlend (Game|GetPlayerController 0) (Variables|Default|GetMainCam) 1.0 "VTBlend_Linear" 0.0 false)
        (Variables|Default|SetInCamera true)))))

(event Input|KeyboardEvents|P
  (params (Key :type Key%20Structure))
  ;[0.9957 0 1] Access
  (:Pressed
    (Utilities|Casting|CastToMain (Game|GetPlayerCharacter 0))))

(fn ConstructionScript)